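; BP_SpawnEnemies is a spawner actor that populates a box volume with random enemies when play begins.
; BeginPlay loops over EnemyCount, spawning a class picked from the Enemies array at a random point inside the Box component bounds.
; Spawns adjust for collisions but always happen.
; The random index range includes the array length, so a pick can fall past the last entry.
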(event EventBeginPlay
  (bind _enemies (Variables|Default|GetEnemies))
  (bind _box (Variables|Default|GetBox))
  (bind (_origin _boxextent) (Collision|GetComponentBounds _box))
  (for _index (range 0 (Variables|Default|GetEnemyCount))
    (Game|SpawnActorfromClass (Utilities|Array|Get(acopy) _enemies (Math|Random|RandomIntegerinRange 0 (Utilities|Array|Length _enemies))) (Math|Conversions|ToTransform(Vector) (Math|Random|RandomPointinBoundingBox _origin _boxextent)) "AdjustIfPossibleButAlwaysSpawn" 0 0)))

(event Collision|EventActorBeginOverlap
  (params (OtherActor :type Actor%20Object%20Reference)))

(event EventTick
  (params (DeltaSeconds :type Float%20%28single-precision%29)))

(fn ConstructionScript)