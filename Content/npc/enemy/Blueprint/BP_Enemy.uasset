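; Base enemy character that handles melee attacks, timed debuffs and death, and kills any other BP_Enemy overlapping its capsule.
; Attack deals damage through a forward capsule trace, gated by a timer.
; DebuffEffect applies stun, slow or blindness (disabling AI sight) until a timer reverts it, while repulsion moves the enemy by a timeline lerp relative to the player.
; Death disables collision, stops AI logic and destroys the actor after a delay.
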(event OnComponentBeginOverlap(CapsuleComponent)
  (params (OverlappedComponent :type Primitive%20Component%20Object%20Reference) (OtherActor :type Actor%20Object%20Reference) (OtherComp :type Primitive%20Component%20Object%20Reference) (OtherBodyIndex :type Integer) (bFromSweep :type Boolean) (SweepResult :type Hit%20Result%20Structure%20%28by%20ref%29))
  (bind _asbp_enemy (Utilities|Casting|CastToBP_Enemy OtherActor))
  (CallFunction|OnDeath _asbp_enemy))

(event Custom|OnDeath
  (if (not (Variables|Default|GetIs%20Dead))
    (Collision|SetCollisionEnabled (Variables|Default|GetCapsuleComponent) "NoCollision")
    (Variables|Default|SetIs%20Dead true)
    (AI|Logic|StopLogic (Variables|/Script/AIModule.AIController|GetBrainComponent (AI|GetAIController self)) "")
    (Utilities|FlowControl|Delay 1.2)
    (Actor|DestroyActor)))

(event Custom|timerEnds
  (bind _charactermovement (Variables|Character|GetCharacterMovement))
  (switch Utilities|FlowControl|Switch|SwitchonEnumDebuffEffects (Variables|Default|GetcurrentDebuff)
    (:NewEnumerator0
      ;[1 1 1] stun
      (Pawn|Components|CharacterMovement|SetMovementMode _charactermovement "MOVE_NavWalking" 0))
    (:NewEnumerator1
      ;[1 1 1] slow
      (Variables|/Script/Engine.CharacterMovementComponent|SetMaxWalkSpeed _charactermovement (/ (Variables|/Script/Engine.CharacterMovementComponent|GetMaxWalkSpeed _charactermovement) (Variables|Default|GetslowCoefficient))))
    (:NewEnumerator3
      (CallFunction|BlindEnemy false))))

(event EventBeginPlay)

(event Collision|EventActorBeginOverlap
  (params (OtherActor :type Actor%20Object%20Reference)))

(event EventTick
  (params (DeltaSeconds :type Float%20%28single-precision%29)))

(event EventDebuffEffect
  (params (DebuffType :type EnumDebuffEffects%20Enum :default "NewEnumerator0") (timer :type Float%20%28single-precision%29))
  (bind _charactermovement (Variables|Character|GetCharacterMovement))
  (Variables|Default|SetcurrentDebuff DebuffType)
  (switch Utilities|FlowControl|Switch|SwitchonEnumDebuffEffects DebuffType
    (:NewEnumerator0
      ;[1 1 1] stun
      (Components|Movement|StopMovementImmediately _charactermovement)
      (Utilities|Time|SetTimerbyEvent (delegate Custom|timerEnds) timer :!label _label))
    (:NewEnumerator1
      ;[1 1 1] slow
      (Variables|/Script/Engine.CharacterMovementComponent|SetMaxWalkSpeed _charactermovement (* (Variables|/Script/Engine.CharacterMovementComponent|GetMaxWalkSpeed _charactermovement) (Variables|Default|GetslowCoefficient)))
      (goto _label))
    (:NewEnumerator2
      (bind _newtrack_0 (Timeline|Timeline_0 Play)
        (:Update
          (Transformation|SetActorLocation (Math|Vector|Lerp(Vector) (Transformation|GetActorLocation (Game|Player|GetPlayerPawn 0)) (Transformation|GetActorLocation self) _newtrack_0) false false))))
    (:NewEnumerator3
      (CallFunction|BlindEnemy true)
      (goto _label))))

(fn ConstructionScript)

(fn Attack
  (bind _returnvalue (Transformation|GetActorLocation))
  (bind _returnvalue_2 (Transformation|GetActorForwardVector))
  (bind _radiusattack (Variables|Default|GetradiusAttack))
  (bind _returnvalue_3 (* _returnvalue_2 _radiusattack))
  (bind _returnvalue_4 (+ _returnvalue _returnvalue_3))
  (if (not (Variables|Default|GetIs%20Attacking))
    (Variables|Default|SetIs%20Attacking true)
    (bind _outhit (Class|KismetSystemLibrary|CapsuleTraceSingleforObjects _returnvalue_4 _returnvalue_4 5e+01 25.0 (Utilities|Array|MakeArray "ObjectTypeQuery3") false 0 "ForDuration" true "(R=1.000000,G=0.000000,B=0.000000,A=1.000000)" "(R=0.000000,G=1.000000,B=0.000000,A=1.000000)" 1e+02))
    (Game|Damage|ApplyDamage (.HitActor (Collision|BreakHitResult _outhit)) (Variables|Default|GetbaseDamage) 0 0)
    (Utilities|Time|SetTimerbyEvent (EventDispatchers|CreateEvent :!event EndAttack) (Variables|Default|GetwaitTime))))

(fn EndAttack
  (Variables|Default|SetIs%20Attacking false))

(fn BlindEnemy
  (params (blind :type Boolean))
  ;[1 1 1] blindness
  (bind _asaicd_enemy (Utilities|Casting|CastToAICD_Enemy (AI|GetAIController self)))
  (Class|AIPerceptionComponent|SetSenseEnabled (Class|AIController|GetAIPerceptionComponent _asaicd_enemy) "/Script/AIModule.AISense_Sight" (not blind)))