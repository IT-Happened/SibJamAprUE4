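; Ranged enemy Blueprint whose Attack function fires a hitscan shot at the player with random spread.
; An IsAttacking guard gates a Pawn object line trace from the enemy to random navigable X/Y near the player, at the player's height.
; BaseDamage goes to the hit actor, then a one-shot WaitTime timer starts.
; The trace leaves long-lasting debug lines, and no reset of IsAttacking appears here.
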(event EventBeginPlay)

(fn ConstructionScript)

(fn Attack
  (bind _returnvalue (Game|Player|GetPlayerPawn 0))
  (bind _returnvalue_2 (Transformation|GetActorLocation _returnvalue))
  (bind _randomlocation (Class|NavigationSystemV1|GetRandomPointinNavigableRadius _returnvalue_2 8e+01 0 0))
  (bind (_x _y) (Math|Vector|BreakVector _randomlocation))
  (if (not (Variables|Default|GetIs%20Attacking))
    (Variables|Default|SetIs%20Attacking true)
    (bind _outhit (Collision|LineTraceForObjects (Transformation|GetActorLocation) (Math|Vector|MakeVector _x _y (.Z (Math|Vector|BreakVector _returnvalue_2))) (Utilities|Array|MakeArray "ObjectTypeQuery3") false 0 "ForDuration" true "(R=1.000000,G=0.000000,B=0.000000,A=1.000000)" "(R=0.000000,G=1.000000,B=0.000000,A=1.000000)" 1e+02))
    (Game|Damage|ApplyDamage (.HitActor (Collision|BreakHitResult _outhit)) (Variables|Default|GetbaseDamage) 0 0)
    (Utilities|Time|SetTimerbyEvent (EventDispatchers|CreateEvent :!event EndAttack) (Variables|Default|GetwaitTime))))