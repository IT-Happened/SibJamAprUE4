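; BP_Quest_1 is a quest Blueprint that defines "A long way home (kill 10 rats)".
; It constructs an order-required BP_ObjectCollection as the root, then adds a single BP_ObjectReachDestination objective targeting MegatonTrigger, labelled "reach Megaton (reach podval)".
; Despite the quest title, no kill objective is created here.
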(fn ConstructionScript
  (|CallParentFunction))

(fn ConstructRootObjectiveCollection
  (bind _returnvalue (Game|ConstructObjectfromClass "/Game/Game/quests/objectieves/BP_ObjectCollection.BP_ObjectCollection_C" self true "A long way home (kill 10 rats)"))
  (return _returnvalue))

(fn PopulateObjectives
  (params (RootObjectCollection :type BP%20Object%20Collection%20Object%20Reference))
  (bind _returnvalue (Game|ConstructObjectfromClass "/Game/Game/quests/objectieves/BP_ObjectReachDestination.BP_ObjectReachDestination_C" self (Variables|Default|GetMegatonTrigger) "reach Megaton (reach podval)"))
  (Default|AddObjective RootObjectCollection _returnvalue))