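; BP_Quest is a base quest Blueprint that owns a root objective collection and starts it when play begins.
; On BeginPlay it constructs and stores the root collection, passes it to PopulateObjectives, then activates it.
; The construct and populate functions are placeholders that only print red debug messages, apparently meant for child quests to override.
; A getter exposes the stored root collection.
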(event EventBeginPlay
  (bind _rootobjectcollection (Private|ConstructRootObjectiveCollection))
  (bind _output_get (Variables|Private|SetRootObjectiveCollection _rootobjectcollection))
  (Private|PopulateObjectives _output_get)
  (Default|ActivateObjective (Variables|Private|GetRootObjectiveCollection)))

(fn ConstructionScript)

(fn ConstructRootObjectiveCollection
  (Development|PrintString "CreateRootObjectiveCollection" true true "(R=1.000000,G=0.062871,B=0.000000,A=1.000000)")
  (return 0))

(fn PopulateObjectives
  (params (RootObjectCollection :type BP%20Object%20Collection%20Object%20Reference))
  (Development|PrintString "CreateRootObjectiveCollection Call For Base Class" true true "(R=1.000000,G=0.062871,B=0.000000,A=1.000000)"))

(fn GetRootObjectiveCollection
  (return (Variables|Private|GetRootObjectiveCollection)))