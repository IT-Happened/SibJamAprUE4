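; BP_Quest_2 is a quest whose root objective is lighting a path, with a name noting it may change to killing mobs.
; It overrides construction of a root BP_ObjectCollection, then populates it with one BP_ObjectLight_Kill objective per entry in Lights.
; Each child objective receives its light reference and a numbered "Turn on light" name.
; The event graph holds only disabled default nodes.
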(event EventBeginPlay
  (|CallParentFunction) ; This node is disabled and will not be called.\nDrag off pins to build functionality.
)

(event Collision|EventActorBeginOverlap
  (params (OtherActor :type Actor%20Object%20Reference)))

(event EventTick
  (params (DeltaSeconds :type Float%20%28single-precision%29)))

(fn ConstructionScript
  (|CallParentFunction))

(fn ConstructRootObjectiveCollection
  (bind _returnvalue (Game|ConstructObjectfromClass "/Game/Game/quests/objectieves/BP_ObjectCollection.BP_ObjectCollection_C" self false "Lighting a path (changes in quest2, may use for killing mobs)"))
  (return _returnvalue))

(fn PopulateObjectives
  (params (RootObjectCollection :type BP%20Object%20Collection%20Object%20Reference))
  (for (_array_element _array_index) (Variables|Default|GetLights)
    (bind _returnvalue (Game|ConstructObjectfromClass "/Game/Game/quests/objectieves/BP_ObjectLight_Kill.BP_ObjectLight_Kill_C" self _array_element (Utilities|Text|FormatText "Turn on light {index}" (+ _array_index 1))))
    (Default|AddObjective RootObjectCollection _returnvalue)))