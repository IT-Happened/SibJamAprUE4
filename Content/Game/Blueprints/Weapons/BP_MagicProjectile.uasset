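; Magic projectile that deals damage on overlap with any actor other than its owner or itself, then destroys itself.
; For each key in the MagicChargePercentage map, it applies a separate hit using that value as base damage and the matching DamageType map entry as damage class.
; The owner is the damage causer, and its Character controller is the instigator.
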(event OnComponentBeginOverlap(Collision)
  (params (OverlappedComponent :type Primitive%20Component%20Object%20Reference) (OtherActor :type Actor%20Object%20Reference) (OtherComp :type Primitive%20Component%20Object%20Reference) (OtherBodyIndex :type Integer) (bFromSweep :type Boolean) (SweepResult :type Hit%20Result%20Structure%20%28by%20ref%29))
  (bind _returnvalue (Components|GetOwner))
  (if (and (!= OtherActor (Components|GetOwner)) (!= self OtherActor))
    (bind _keys (Utilities|Map|Keys (Variables|Default|GetMagicChargePercentage)))
    (for _array_element _keys
      (Game|Damage|ApplyDamage OtherActor (.Value (Utilities|Map|Find (Variables|Default|GetMagicChargePercentage) _array_element)) (Pawn|GetController (.AsCharacter (Utilities|Casting|CastToCharacter _returnvalue))) _returnvalue (.Value (Utilities|Map|Find (Variables|Default|GetDamageType) _array_element))))
    (Actor|DestroyActor)))

(fn ConstructionScript)