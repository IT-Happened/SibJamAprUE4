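; Magic weapon that charges a stack of element powers, capped at 100 in total, and releases it as spells.
; A looping timer drives charging, growing the last element or merging a differing one through DT_ElementCombinations, otherwise appending it.
; On release, adjacent pairs matching DT_SkillsCombintaions, which allows a wildcard element, spawn and use BP_Skill subclasses and are removed from the stack.
; BP_MagicProjectile then spawns with the remaining charge, while dispelling simply clears it.
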(fn ConstructionScript)

(fn StartChargingMagic
  (Variables|Default|SetbCharging true)
  (bind _returnvalue (Utilities|Time|SetTimerbyEvent (EventDispatchers|CreateEvent :!event ChargeMagic) 0.1 true))
  (Variables|Timers|SetChargeTimer _returnvalue))

(fn ReleaseMagic
  (params (Location :type Vector) (Direction :type Rotator))
  (if (Variables|Default|GetbCharging)
    (Variables|Default|SetbCharging false)
    (Utilities|Time|ClearandInvalidateTimerbyHandle (Variables|Timers|GetChargeTimer))
    (CallFunction|CalculateSkills)
    (Game|SpawnActorfromClass "/Game/Game/Blueprints/Weapons/BP_MagicProjectile.BP_MagicProjectile_C" (Math|Transform|MakeTransform Location Direction) "AlwaysSpawn" (Components|GetOwner) (Variables|Default|GetMagicChargePercentage) 0)
    (Utilities|Array|Clear (Variables|Default|GetMagicChargePercentage))))

(fn ChargeMagic
  (bind _magicchargepercentage (Variables|Default|GetMagicChargePercentage))
  (bind _magicchargepercentage_2 (Variables|Default|GetMagicChargePercentage))
  (bind _returnvalue (Utilities|Array|LastIndex _magicchargepercentage_2))
  (bind _output (Utilities|Array|Get(acopy) _magicchargepercentage_2 _returnvalue))
  (bind (_element _power) (Utilities|Struct|BreakS_ElementPower _output))
  (if (< (CallFunction|GetAllPercentage) 1e+02)
    (if (> (Utilities|Array|Length (Variables|Default|GetMagicChargePercentage)) 0)
      (if (Utilities|Enum|Equal(Enum) (.Element (Utilities|Struct|BreakS_ElementPower (Utilities|Array|Get(acopy) _magicchargepercentage (Utilities|Array|LastIndex _magicchargepercentage)))) (Variables|Default|GetCurrentMagicElement))
        (|SetBy-RefVar _output (Utilities|Struct|MakeS_ElementPower _element (+ _power (Math|Float|Clamp(Float) (* (Class|KismetSystemLibrary|GetTimerElapsedTimeHandle (Variables|Timers|GetChargeTimer)) (Variables|Default|GetChargeMultiplayer)) 0.0 (- 1e+02 (CallFunction|GetAllPercentage))))))
        (else
          (bind _found (CallFunction|FindElementtoCombine))
          (if (not _found)
            (Utilities|Array|Add (Variables|Default|GetMagicChargePercentage) (Utilities|Struct|MakeS_ElementPower (Variables|Default|GetCurrentMagicElement) (* (Class|KismetSystemLibrary|GetTimerElapsedTimeHandle (Variables|Timers|GetChargeTimer)) (Variables|Default|GetChargeMultiplayer))) :!label _label))))
      (else
        (goto _label)))))

(fn GetAllPercentage
  (for _array_element (Variables|Default|GetMagicChargePercentage)
    (LocalVariables|SetPercentage (+ (LocalVariables|GetPercentage) (.Power (Utilities|Struct|BreakS_ElementPower _array_element)))))
  (return (LocalVariables|GetPercentage)))

(fn DispelMagic
  (Variables|Default|SetbCharging false)
  (Utilities|Time|ClearandInvalidateTimerbyHandle (Variables|Timers|GetChargeTimer))
  (Utilities|Array|Clear (Variables|Default|GetMagicChargePercentage)))

(fn CalculateSkills
  (bind _magicchargepercentage (Variables|Default|GetMagicChargePercentage))
  (for (_array_element _array_index) _magicchargepercentage
    (if (!= _array_index (Utilities|Array|LastIndex _magicchargepercentage))
      (LocalVariables|Set_Element1 _array_element)
      (LocalVariables|Set_Element2 (Utilities|Array|Get(acopy) _magicchargepercentage (+ _array_index 1)))
      (bind _outrownames (DataTable|GetDataTableRowNames "/Game/Game/Data/DataTables/DT_SkillsCombintaions.DT_SkillsCombintaions"))
      (for _array_element_2 _outrownames
        (bind _returnvalue (Utilities|GetDataTableRow "/Game/Game/Data/DataTables/DT_SkillsCombintaions.DT_SkillsCombintaions" _array_element_2)
          (:then
            (bind _output_get (LocalVariables|SetCombo _returnvalue))
            (if (or (and (or (Utilities|Enum|Equal(Enum) (.Element1 (Utilities|Struct|BreakS_SkillsCombinations _output_get)) (.Element (Utilities|Struct|BreakS_ElementPower (LocalVariables|Get_Element1)))) (Utilities|Enum|Equal(Enum) (.Element1 (Utilities|Struct|BreakS_SkillsCombinations _output_get)) "NewEnumerator11")) (or (Utilities|Enum|Equal(Enum) (.Element2 (Utilities|Struct|BreakS_SkillsCombinations _output_get)) (.Element (Utilities|Struct|BreakS_ElementPower (LocalVariables|Get_Element2)))) (Utilities|Enum|Equal(Enum) (.Element2 (Utilities|Struct|BreakS_SkillsCombinations _output_get)) "NewEnumerator11"))) (and (or (Utilities|Enum|Equal(Enum) (.Element2 (Utilities|Struct|BreakS_SkillsCombinations _output_get)) (.Element (Utilities|Struct|BreakS_ElementPower (LocalVariables|Get_Element1)))) (Utilities|Enum|Equal(Enum) (.Element2 (Utilities|Struct|BreakS_SkillsCombinations _output_get)) "NewEnumerator11")) (or (Utilities|Enum|Equal(Enum) (.Element1 (Utilities|Struct|BreakS_SkillsCombinations _output_get)) (.Element (Utilities|Struct|BreakS_ElementPower (LocalVariables|Get_Element2)))) (Utilities|Enum|Equal(Enum) (.Element1 (Utilities|Struct|BreakS_SkillsCombinations _output_get)) "NewEnumerator11"))))
              (bind _returnvalue_2 (Utilities|LoadClassAssetBlocking (.Skill (Utilities|Struct|BreakS_SkillsCombinations _output_get))))
              (bind _asbp_skill (Utilities|Casting|CastToBP_SkillClass _returnvalue_2))
              (bind _returnvalue_3 (Game|SpawnActorfromClass _asbp_skill (Math|Transform|MakeTransform "0, 0,0.000000") "AlwaysSpawn" (Components|GetOwner) 0))
              (Default|UseSkill _returnvalue_3 (select (Utilities|Enum|Equal(Enum) (.Element1 (Utilities|Struct|BreakS_SkillsCombinations (LocalVariables|GetCombo))) (.Element (Utilities|Struct|BreakS_ElementPower (LocalVariables|Get_Element1)))) (.Power (Utilities|Struct|BreakS_ElementPower (LocalVariables|Get_Element1))) (.Power (Utilities|Struct|BreakS_ElementPower (LocalVariables|Get_Element2)))) (select (Utilities|Enum|Equal(Enum) (.Element2 (Utilities|Struct|BreakS_SkillsCombinations (LocalVariables|GetCombo))) (.Element (Utilities|Struct|BreakS_ElementPower (LocalVariables|Get_Element2)))) (.Power (Utilities|Struct|BreakS_ElementPower (LocalVariables|Get_Element2))) (.Power (Utilities|Struct|BreakS_ElementPower (LocalVariables|Get_Element1)))))
              (Utilities|Array|RemoveItem (Variables|Default|GetMagicChargePercentage) (LocalVariables|Get_Element1))
              (Utilities|Array|RemoveItem (Variables|Default|GetMagicChargePercentage) (LocalVariables|Get_Element2)))))))))

(fn FindElementtoCombine
  (bind _magicchargepercentage (Variables|Default|GetMagicChargePercentage))
  (bind _magicchargepercentage_2 (Variables|Default|GetMagicChargePercentage))
  (bind _returnvalue (Utilities|Array|LastIndex _magicchargepercentage))
  (bind _returnvalue_2 (Utilities|Array|LastIndex _magicchargepercentage_2))
  (bind _output (Utilities|Array|Get(acopy) _magicchargepercentage _returnvalue))
  (bind _output_2 (Utilities|Array|Get(acopy) _magicchargepercentage_2 _returnvalue_2))
  (bind _element (Utilities|Struct|BreakS_ElementPower _output_2))
  (bind _outrownames (DataTable|GetDataTableRowNames "/Game/Game/Data/DataTables/DT_ElementCombinations.DT_ElementCombinations"))
  (for _array_element _outrownames
    (bind _returnvalue_3 (Utilities|GetDataTableRow "/Game/Game/Data/DataTables/DT_ElementCombinations.DT_ElementCombinations" _array_element)
      (:then
        (if (or (and (Utilities|Enum|Equal(Enum) (.Element1 (Utilities|Struct|BreakS_ElementCombitanions _returnvalue_3)) (Variables|Default|GetCurrentMagicElement)) (Utilities|Enum|Equal(Enum) (.Element2 (Utilities|Struct|BreakS_ElementCombitanions _returnvalue_3)) _element)) (and (Utilities|Enum|Equal(Enum) (.Element2 (Utilities|Struct|BreakS_ElementCombitanions _returnvalue_3)) (Variables|Default|GetCurrentMagicElement)) (Utilities|Enum|Equal(Enum) (.Element1 (Utilities|Struct|BreakS_ElementCombitanions _returnvalue_3)) _element)))
          (bind _output_get (Variables|Default|SetCurrentMagicElement (.Final (Utilities|Struct|BreakS_ElementCombitanions _returnvalue_3))))
          (|SetBy-RefVar _output (Utilities|Struct|MakeS_ElementPower _output_get (.Power (Utilities|Struct|BreakS_ElementPower _output))))
          (return true)))))
  (return false))