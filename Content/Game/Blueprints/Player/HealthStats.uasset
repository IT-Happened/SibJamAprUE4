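; HealthStats holds a player's max and current HP and MP for display on the HUD.
; A setter function overwrites all four values at once.
; A getter returns each value as truncated integer text, along with HP and MP progress-bar fractions normalized from zero to their maximums.
; It only stores and formats data, with no active event logic or clamping.
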(event EventBeginPlay)

(event EventTick
  (params (DeltaSeconds :type Float%20%28single-precision%29)))

(fn GetStatsforHUD
  (return (Utilities|Text|ToText(Integer) (Math|Float|Truncate (Variables|Default|GetMax_HP))) (Utilities|Text|ToText(Integer) (Math|Float|Truncate (Variables|Default|GetCurrent_HP))) (Math|Float|NormalizetoRange (Variables|Default|GetCurrent_HP) 0.0 (Variables|Default|GetMax_HP)) (Utilities|Text|ToText(Integer) (Math|Float|Truncate (Variables|Default|GetMax_MP))) (Utilities|Text|ToText(Integer) (Math|Float|Truncate (Variables|Default|GetCurrent_MP))) (Math|Float|NormalizetoRange (Variables|Default|GetCurrent_MP) 0.0 (Variables|Default|GetMax_MP))))

(fn SetHPandMP
  (params (Set%20Max%20HP :type Float%20%28single-precision%29) (Set%20Current%20HP :type Float%20%28single-precision%29) (Set%20Max%20MP :type Float%20%28single-precision%29) (Set%20Current%20MP :type Float%20%28single-precision%29))
  (Variables|Default|SetMax_HP Set%20Max%20HP)
  (Variables|Default|SetCurrent_HP Set%20Current%20HP)
  (Variables|Default|SetMax_MP Set%20Max%20MP)
  (Variables|Default|SetCurrent_MP Set%20Current%20MP))