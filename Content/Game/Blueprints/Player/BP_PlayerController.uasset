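; Player controller that opens the game's menu screens from keyboard shortcuts.
; P, M and L each cast the game instance to MainGameInstance and call it to show the pause menu, map or diary.
; On BeginPlay it sets game-only input mode so play starts without a cursor.
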(event EventBeginPlay
  ;[1 1 1] Запуск игры без курсора
  (Input|SetInputModeGameOnly self))

(event Input|KeyboardEvents|P
  (params (Key :type Key%20Structure :default "None"))
  ;[1 1 1] Показ меню паузы по нажатию p
  (:Pressed
    (bind _asmain_game_instance (Utilities|Casting|CastToMainGameInstance (Game|GetGameInstance)))
    (Default|ShowPauseMenu _asmain_game_instance)))

(event Input|KeyboardEvents|M
  (params (Key :type Key%20Structure :default "None"))
  ;[1 1 1] Показ карты по нажатию m
  (:Pressed
    (bind _asmain_game_instance (Utilities|Casting|CastToMainGameInstance (Game|GetGameInstance)))
    (Default|ShowMap _asmain_game_instance)))

(event Input|KeyboardEvents|L
  (params (Key :type Key%20Structure :default "None"))
  ;[1 1 1] Показ дневника по нажатию l
  (:Pressed
    (bind _asmain_game_instance (Utilities|Casting|CastToMainGameInstance (Game|GetGameInstance)))
    (Default|ShowDiary _asmain_game_instance)))

(fn ConstructionScript)