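; Enemy character Blueprint with a health component and a widget component that displays its stats.
; On begin play it binds to the health component's damage event and forwards current and max health to the WBP_EnemyStats widget.
; A LockTarget event shows the widget while the enemy is targeted and hides it otherwise.
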(event Custom|OnDamage
  (params (CurrentHealth :type Float%20%28single-precision%29) (MaxHealth :type Float%20%28single-precision%29))
  (bind _aswbp_enemy_stats (Utilities|Casting|CastToWBP_EnemyStats (UserInterface|GetWidget (Variables|Default|GetWidget))))
  (Default|TakeDamage _aswbp_enemy_stats CurrentHealth MaxHealth))

(event EventLockTarget
  (params (On :type Boolean))
  (Development|SetHiddeninGame (Variables|Default|GetWidget) (not On) false))

(event EventBeginPlay
  (|CallParentFunction)
  (EventDispatchers|BindEventtoDamage (Variables|Default|GetBP_HealthComponent) (delegate Custom|OnDamage)))

(fn ConstructionScript
  (|CallParentFunction))