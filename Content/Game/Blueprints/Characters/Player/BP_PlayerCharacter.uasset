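; Player character with movement, automatic enemy lock-on and elemental magic casting.
; A looping timer finds the nearest living enemy within range, enabling battle mode and its walk speed, while a second timer releases dead or out-of-range targets.
; While locked, Tick interpolates the camera toward the target with clamped pitch, and ChangeTarget picks a different random enemy.
; Charge, release and element inputs are forwarded to the magic component.
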(event Custom|FindTargets
  (Utilities|IsValid (Variables|Targeting|GetTargetedEnemy)
    (:Is%20Not%20Valid
      (bind _targets (CallFunction|FindEnemies))
      (bind _output_get (Variables|Targeting|SetTargetedEnemy (CallFunction|SelectTarget _targets)))
      (Utilities|IsValid _output_get
        (:Is%20Valid
          (CallFunction|LockonTarget)
          (bind _returnvalue (Utilities|Time|SetTimerbyEvent (delegate Custom|CheckInRange) 0.1 true))
          (Variables|Targeting|SetRangeCheckTimer _returnvalue)
          (CallFunction|EnableBattleMode))
        (:Is%20Not%20Valid
          (if (Variables|Targeting|GetbCameraLocked)
            (CallFunction|ResetCameraLock)))))))

(event Custom|LockOnTarget
  (Variables|Targeting|SetbCameraLocked true)
  (Class|BICharacterInterface|LockTarget(Message) (Variables|Targeting|GetTargetedEnemy) true))

(event Custom|ResetCameraLock
  (Variables|Targeting|SetbCameraLocked false))

(event Custom|CheckInRange
  (if (not (CallFunction|CheckTarget))
    (CallFunction|ResetTargeting)))

(event Custom|ResetTargeting
  (Class|BICharacterInterface|LockTarget(Message) (Variables|Targeting|GetTargetedEnemy) false)
  (CallFunction|ResetCameraLock)
  (Variables|Targeting|SetTargetedEnemy 0)
  (Utilities|Time|ClearandInvalidateTimerbyHandle (Variables|Targeting|GetRangeCheckTimer))
  (CallFunction|DisableBattleMode))

(event Custom|EnableBattleMode
  (Variables|Targeting|SetbBattleMod true)
  (CallFunction|ResetCharacterSpeed))

(event Custom|DisableBattleMode
  (Variables|Targeting|SetbBattleMod false)
  (CallFunction|ResetCharacterSpeed))

(event EventBeginPlay
  (Utilities|Time|SetTimerbyEvent (delegate Custom|FindTargets) 0.1 true))

(event EventTick
  (params (DeltaSeconds :type Float%20%28single-precision%29))
  (Utilities|FlowControl|Sequence
    (:then_0
      (if (Variables|Targeting|GetbCameraLocked)
        (CallFunction|LockCamera)))))

(event Input|ActionEvents|InputActionChangeTarget
  (params (Key :type Key%20Structure))
  (:Pressed
    (if (Variables|Targeting|GetbBattleMod)
      (CallFunction|ChangeTarget))))

(event Input|AxisEvents|InputAxisMoveForward
  (params (AxisValue :type Float%20%28single-precision%29))
  ;[1 1 1] Controls
  (Pawn|Input|AddMovementInput (Transformation|GetActorForwardVector) AxisValue false))

(event Input|AxisEvents|InputAxisMoveRight
  (params (AxisValue :type Float%20%28single-precision%29))
  ;[1 1 1] Controls
  (Pawn|Input|AddMovementInput (Transformation|GetActorRightVector) AxisValue false))

(event Input|AxisEvents|InputAxisLookVertical
  (params (AxisValue :type Float%20%28single-precision%29))
  ;[1 1 1] Controls
  (if (not (Variables|Targeting|GetbCameraLocked))
    (Pawn|Input|AddControllerPitchInput AxisValue)))

(event Input|AxisEvents|InputAxisLookHorizontal
  (params (AxisValue :type Float%20%28single-precision%29))
  ;[1 1 1] Controls
  (if (not (Variables|Targeting|GetbCameraLocked))
    (Pawn|Input|AddControllerYawInput AxisValue)))

(event Input|ActionEvents|InputActionChargeMagic
  (params (Key :type Key%20Structure))
  (:Pressed
    (Class|MagicComponent|StartChargeMagic (Variables|Default|GetBP_MagicComponent)))
  (:Released
    (Class|MagicComponent|ReleaseMagic (Variables|Default|GetBP_MagicComponent))))

(event Input|ActionEvents|InputActionFireElement
  (params (Key :type Key%20Structure))
  (:Pressed
    (Class|MagicComponent|ChangeMagicElement (Variables|Default|GetBP_MagicComponent) "ME_Fire")))

(event Input|ActionEvents|InputActionWaterElement
  (params (Key :type Key%20Structure))
  (:Pressed
    (Class|MagicComponent|ChangeMagicElement (Variables|Default|GetBP_MagicComponent) "ME_Water")))

(event Input|ActionEvents|InputActionEarthElement
  (params (Key :type Key%20Structure))
  (:Pressed
    (Class|MagicComponent|ChangeMagicElement (Variables|Default|GetBP_MagicComponent) "ME_Earth")))

(event Input|ActionEvents|InputActionWindElement
  (params (Key :type Key%20Structure))
  (:Pressed
    (Class|MagicComponent|ChangeMagicElement (Variables|Default|GetBP_MagicComponent) "ME_Wind")))

(event Input|ActionEvents|InputActionLightElement
  (params (Key :type Key%20Structure))
  (:Pressed
    (Class|MagicComponent|ChangeMagicElement (Variables|Default|GetBP_MagicComponent) "ME_Light")))

(event Input|ActionEvents|InputActionDarkElement
  (params (Key :type Key%20Structure))
  (:Pressed
    (Class|MagicComponent|ChangeMagicElement (Variables|Default|GetBP_MagicComponent) "ME_Dark")))

(fn ConstructionScript)

(fn SelectTarget
  (params (Targets :type Array%20of%20Actor%20Object%20References))
  (if (> (Utilities|Array|Length Targets) 0)
    (LocalVariables|SetDistance (Variables|Targeting|GetTargetArea))
    (for _array_element Targets
      (bind _output_get (LocalVariables|SetDistanceToEnemy (Transformation|GetDistanceTo self _array_element)))
      (if (< _output_get (LocalVariables|GetDistance))
        (LocalVariables|SetDistance (LocalVariables|GetDistanceToEnemy))
        (LocalVariables|Set_Target _array_element)))
    (return (LocalVariables|Get_Target))
    (else
      (return 0))))

(fn CheckTarget
  (return (and (not (Variables|/Game/Game/Blueprints/Components/BP_HealthComponent.BP_HealthComponent_C|GetbIsDead (Actor|GetComponentbyClass (Variables|Targeting|GetTargetedEnemy) "/Game/Game/Blueprints/Components/BP_HealthComponent.BP_HealthComponent_C"))) (<= (Transformation|GetDistanceTo self (Variables|Targeting|GetTargetedEnemy)) (Variables|Targeting|GetTargetArea)))))

(fn LockCamera
  (bind _returnvalue (Pawn|GetController))
  (bind _targetedenemy (Variables|Targeting|GetTargetedEnemy))
  (bind _returnvalue_2 (Transformation|GetActorLocation _targetedenemy))
  (bind _asplayer_controller (Utilities|Casting|CastToPlayerController _returnvalue))
  (bind _playercameramanager (Variables|/Script/Engine.PlayerController|GetPlayerCameraManager _asplayer_controller))
  (bind _returnvalue_3 (Camera|GetCameraLocation _playercameramanager))
  (bind _returnvalue_4 (Math|Rotator|FindLookatRotation _returnvalue_3 _returnvalue_2))
  (bind (_roll _pitch _yaw) (Math|Rotator|BreakRotator _returnvalue_4))
  (bind _output_get (LocalVariables|SetTargetRotation (Math|Rotator|MakeRotator 0.0 (Math|Float|ClampAngle (- _pitch 5.0) -25.0 0.0) _yaw)))
  (Pawn|SetControlRotation _returnvalue (Math|Interpolation|RInterpTo (Camera|GetCameraRotation _playercameramanager) _output_get (Utilities|Time|GetWorldDeltaSeconds) 9.0)))

(fn ChangeTarget
  (bind _targets (CallFunction|FindEnemies))
  (if (> (Utilities|Array|Length _targets) 1)
    (bind _output_get (LocalVariables|SetTarget (Utilities|Array|Get(acopy) _targets (Math|Random|RandomInteger (Utilities|Array|Length _targets))) :!label _label))
    (if (!= _output_get (Variables|Targeting|GetTargetedEnemy))
      (Class|BICharacterInterface|LockTarget(Message) (Variables|Targeting|GetTargetedEnemy) false)
      (Variables|Targeting|SetTargetedEnemy (LocalVariables|GetTarget))
      (CallFunction|LockonTarget)
      (else
        (goto _label)))))

(fn ResetCharacterSpeed
  (Variables|/Script/Engine.CharacterMovementComponent|SetMaxWalkSpeed (Variables|Character|GetCharacterMovement) (Math|Float|SelectFloat (Math|Float|SelectFloat (Variables|Default|GetMaxChargingSpeed) (Variables|Default|GetMaxBattleSpeed) false) (Variables|Default|GetMaxSpeed) (Variables|Targeting|GetbBattleMod))))

(fn ChoseTargetArrays
  (params (Array :type Array%20of%20Actor%20Object%20References))
  (for _array_element Array
    (if (not (Variables|/Game/Game/Blueprints/Components/BP_HealthComponent.BP_HealthComponent_C|GetbIsDead (Actor|GetComponentbyClass _array_element "/Game/Game/Blueprints/Components/BP_HealthComponent.BP_HealthComponent_C")))
      (Utilities|Array|Add (LocalVariables|Get_Targets) _array_element)))
  (return (LocalVariables|Get_Targets)))

(fn FindEnemies
  (bind _outactors (Collision|SphereOverlapActors (Transformation|GetActorLocation) (Variables|Targeting|GetTargetArea) (Utilities|Array|MakeArray "ObjectTypeQuery3") "/Game/Game/Blueprints/Characters/Enemy/BP_EnemyCharacter.BP_EnemyCharacter_C"))
  (bind _targets (CallFunction|ChoseTargetArrays _outactors))
  (return _targets))