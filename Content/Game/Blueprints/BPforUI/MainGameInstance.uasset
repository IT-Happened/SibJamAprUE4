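; Game instance that manages the pause menu, map, diary, settings and credits UI.
; Show events lazily create and cache each widget; pause menu, map and diary also pause the game, show the cursor and set input focus, while their resume events restore gameplay.
; Opening a screen removes competing widgets, but multi-widget cleanup uses nested validity checks, so later removals run only if earlier widgets exist.
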(event Custom|PauseMenuResume
  (bind _returnvalue (Game|GetPlayerController 0))
  ;[1 1 1] Возращение к игре из меню паузы (и закрытие меню настроек, авторов)
  (Widget|RemovefromParent (Variables|Widgets|GetPauseMenuWB))
  (Game|SetGamePaused false)
  (Input|SetInputModeGameOnly _returnvalue)
  (Variables|/Script/Engine.PlayerController|SetbShowMouseCursor _returnvalue false)
  (bind _settingswb (Variables|Widgets|GetSettingsWB)
    (:then
      (Widget|RemovefromParent _settingswb)
      (bind _creditswb (Variables|Widgets|GetCreditsWB)
        (:then
          (Widget|RemovefromParent _creditswb))
        (:else)))
    (:else)))

(event Custom|ShowCredits
  ;[1 1 1] Показ списка разработчиков (и закрываем меню настроек, если было открыто)
  (Utilities|IsValid (Variables|Widgets|GetCreditsWB)
    (:Is%20Valid
      _)
    (:Is%20Not%20Valid
      (bind _returnvalue (UserInterface|CreateWidget "/Game/Game/UI/Menus/CreditsMenuWB.CreditsMenuWB_C" (Game|GetPlayerController 0)))
      (Variables|Widgets|SetCreditsWB _returnvalue)))
  (UserInterface|Viewport|AddtoViewport (Variables|Widgets|GetCreditsWB) 0)
  (bind _settingswb (Variables|Widgets|GetSettingsWB)
    (:then
      (Widget|RemovefromParent _settingswb))
    (:else)))

(event Custom|ShowMap
  (bind _returnvalue (Game|GetPlayerController 0))
  ;[1 1 1] Вызываем карту и показываем курсор (и закрываем меню или дневник если были открыты)
  (Utilities|IsValid (Variables|Widgets|GetMapWB)
    (:Is%20Valid
      _)
    (:Is%20Not%20Valid
      (bind _returnvalue_2 (UserInterface|CreateWidget "/Game/Game/UI/Menus/MapLowerWB.MapLowerWB_C" _returnvalue))
      (Variables|Widgets|SetMapWB _returnvalue_2)))
  (UserInterface|Viewport|AddtoViewport (Variables|Widgets|GetMapWB) 0)
  (Game|SetGamePaused true)
  (Variables|/Script/Engine.PlayerController|SetbShowMouseCursor _returnvalue true)
  (Input|SetInputModeUIOnly _returnvalue (Variables|Widgets|GetMapWB) "LockInFullscreen")
  (bind _diarywb (Variables|Widgets|GetDiaryWB)
    (:then
      (Widget|RemovefromParent _diarywb)
      (bind _pausemenuwb (Variables|Widgets|GetPauseMenuWB)
        (:then
          (Widget|RemovefromParent _pausemenuwb)
          (bind _settingswb (Variables|Widgets|GetSettingsWB)
            (:then
              (Widget|RemovefromParent _settingswb)
              (bind _creditswb (Variables|Widgets|GetCreditsWB)
                (:then
                  (Widget|RemovefromParent _creditswb))
                (:else)))
            (:else)))
        (:else)))
    (:else)))

(event Custom|ResumeMap
  (bind _returnvalue (Game|GetPlayerController 0))
  ;[1 1 1] Возращение к игре из карты
  (Widget|RemovefromParent (Variables|Widgets|GetMapWB))
  (Game|SetGamePaused false)
  (Input|SetInputModeGameOnly _returnvalue)
  (Variables|/Script/Engine.PlayerController|SetbShowMouseCursor _returnvalue false))

(event Custom|ShowDiary
  (bind _returnvalue (Game|GetPlayerController 0))
  ;[1 1 1] Вызываем дневник и показываем курсор (и закрываем меню или карту если были открыты)
  (Utilities|IsValid (Variables|Widgets|GetDiaryWB)
    (:Is%20Valid
      _)
    (:Is%20Not%20Valid
      (bind _returnvalue_2 (UserInterface|CreateWidget "/Game/Game/UI/Menus/DiaryLowerWB.DiaryLowerWB_C" _returnvalue))
      (Variables|Widgets|SetDiaryWB _returnvalue_2)))
  (UserInterface|Viewport|AddtoViewport (Variables|Widgets|GetDiaryWB) 0)
  (Game|SetGamePaused true)
  (Variables|/Script/Engine.PlayerController|SetbShowMouseCursor _returnvalue true)
  (Input|SetInputModeUIOnly _returnvalue (Variables|Widgets|GetDiaryWB) "LockInFullscreen")
  (bind _mapwb (Variables|Widgets|GetMapWB)
    (:then
      (Widget|RemovefromParent _mapwb)
      (bind _pausemenuwb (Variables|Widgets|GetPauseMenuWB)
        (:then
          (Widget|RemovefromParent _pausemenuwb)
          (bind _settingswb (Variables|Widgets|GetSettingsWB)
            (:then
              (Widget|RemovefromParent _settingswb)
              (bind _creditswb (Variables|Widgets|GetCreditsWB)
                (:then
                  (Widget|RemovefromParent _creditswb))
                (:else)))
            (:else)))
        (:else)))
    (:else)))

(event Custom|ShowPauseMenu
  (bind _returnvalue (Game|GetPlayerController 0))
  ;[1 1 1] Вызываем меню паузы и показываем курсор (и закрываем дневник или карту если были открыты)
  (Utilities|IsValid (Variables|Widgets|GetPauseMenuWB)
    (:Is%20Valid
      _)
    (:Is%20Not%20Valid
      (bind _returnvalue_2 (UserInterface|CreateWidget "/Game/Game/UI/Menus/PauseMenuLowerWB.PauseMenuLowerWB_C" _returnvalue))
      (Variables|Widgets|SetPauseMenuWB _returnvalue_2)))
  (UserInterface|Viewport|AddtoViewport (Variables|Widgets|GetPauseMenuWB) 0)
  (Game|SetGamePaused true)
  (Variables|/Script/Engine.PlayerController|SetbShowMouseCursor _returnvalue true)
  (Input|SetInputModeGameandUI _returnvalue (Variables|Widgets|GetPauseMenuWB) "LockInFullscreen" false)
  (bind _diarywb (Variables|Widgets|GetDiaryWB)
    (:then
      (Widget|RemovefromParent _diarywb)
      (bind _mapwb (Variables|Widgets|GetMapWB)
        (:then
          (Widget|RemovefromParent _mapwb)
          (bind _settingswb (Variables|Widgets|GetSettingsWB)
            (:then
              (Widget|RemovefromParent _settingswb)
              (bind _creditswb (Variables|Widgets|GetCreditsWB)
                (:then
                  (Widget|RemovefromParent _creditswb))
                (:else)))
            (:else)))
        (:else)))
    (:else)))

(event Custom|ShowSettings
  ;[1 1 1] Вызов меню настроек (и закрываем меню разработчиков, если было открыто)
  (Utilities|IsValid (Variables|Widgets|GetSettingsWB)
    (:Is%20Valid
      _)
    (:Is%20Not%20Valid
      (bind _returnvalue (UserInterface|CreateWidget "/Game/Game/UI/Menus/SettingsMenuWB.SettingsMenuWB_C" (Game|GetPlayerController 0)))
      (Variables|Widgets|SetSettingsWB _returnvalue)))
  (UserInterface|Viewport|AddtoViewport (Variables|Widgets|GetSettingsWB) 0)
  (bind _creditswb (Variables|Widgets|GetCreditsWB)
    (:then
      (Widget|RemovefromParent _creditswb))
    (:else)))

(event Custom|DiaryResume
  (bind _returnvalue (Game|GetPlayerController 0))
  ;[1 1 1] Возращение к игре из дневника
  (Widget|RemovefromParent (Variables|Widgets|GetDiaryWB))
  (Game|SetGamePaused false)
  (Input|SetInputModeGameOnly _returnvalue)
  (Variables|/Script/Engine.PlayerController|SetbShowMouseCursor _returnvalue false))