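; BP_MagicComponent is a magic component that holds a list of element powers and a current magic element.
; Its only active graph logic is a debug readout on Tick, printing each element with its power, then the current element, with zero-duration on-screen strings.
; BeginPlay is an unused stub, and the graph never modifies the magic state.
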(event EventBeginPlay)

(event EventTick
  (params (DeltaSeconds :type Float%20%28single-precision%29))
  (Utilities|FlowControl|Sequence
    (:then_0
      (for _array_element (Variables|Default|GetElementsPowers)
        (Development|PrintString (Utilities|String|Append (Utilities|String|EnumtoString (.Element (Utilities|Struct|BreakElementPower _array_element))) ": " (Utilities|String|ToString(Float) (.Power (Utilities|Struct|BreakElementPower _array_element)))) true true "(R=0.000000,G=0.660000,B=1.000000,A=1.000000)" 0.0)))
    (:then_1
      (Development|PrintString (Utilities|String|Append "Current magic: " (Utilities|String|EnumtoString (Variables|Default|GetCurrentMagicElement))) true true "(R=0.000000,G=0.660000,B=1.000000,A=1.000000)" 0.0))))